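; Collectible coin actor that adds score to the player on touch.
; On BeginPlay it takes a random starting yaw and gives its RotatingMovement component a random spin rate, so coins do not turn in sync.
; When a BP_Player overlaps its Sphere, it passes CoinScoreToAdd to the player's AddScore, plays an explosion sound and particle effect, then destroys itself.
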(event OnComponentBeginOverlap(Sphere)
  (params (OverlappedComponent :type Primitive%20Component%20Object%20Reference) (OtherActor :type Actor%20Object%20Reference) (OtherComp :type Primitive%20Component%20Object%20Reference) (OtherBodyIndex :type Integer) (bFromSweep :type Boolean) (SweepResult :type Hit%20Result%20Structure%20%28by%20ref%29))
  (bind _asbp_player (Utilities|Casting|CastToBP_Player OtherActor))
  (Default|AddScore _asbp_player (Variables|Default|GetCoinScoreToAdd))
  (Audio|PlaySound2D "/Game/StarterContent/Audio/Explosion01.Explosion01" 1.0 1.0 0.0 0 0)
  (Effects|SpawnEmitteratLocation "/Game/StarterContent/Particles/P_Explosion.P_Explosion" (Transformation|GetActorLocation))
  (Actor|DestroyActor))

(event EventBeginPlay
  (Transformation|SetActorRotation (Math|Rotator|MakeRotator 0.0 0.0 (Math|Random|RandomFloatinRange -9e+01 9e+01)))
  (Variables|/Script/Engine.RotatingMovementComponent|SetRotationRate (Variables|Default|GetRotatingMovement) (Math|Rotator|MakeRotator 0.0 0.0 (Math|Random|RandomFloatinRange 1e+02 1.8e+02))))

(fn ConstructionScript)